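; AgroCheck is a behavior tree tick that finds visible targets for an AI follower run by Follower_AI_CON.
; A large multi-sphere trace around the controlled pawn gathers actors of the desired object types.
; Each hit gets a Camera-channel line-of-sight trace, which writes TargetToFollow and TargetLocation when clear, or empties TargetToFollow when blocked.
; The loop never breaks, so the last hit checked decides the target.
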(event EventTick
  (params (OwnerActor :type Actor%20Object%20Reference) (DeltaSeconds :type Float%20%28single-precision%29))
  (bind _asfollower_ai_con (Utilities|Casting|CastToFollower_AI_CON OwnerActor))
  (Variables|Default|SetAI_CON_Ref _asfollower_ai_con)
  (Variables|Default|SetMy%20Location (Transformation|GetActorLocation (Pawn|GetControlledPawn _asfollower_ai_con)))
  (bind _outhits (Collision|MultiSphereTraceForObjects 0 (Transformation|GetActorLocation (Pawn|GetControlledPawn _asfollower_ai_con)) (+ (Transformation|GetActorLocation (Pawn|GetControlledPawn _asfollower_ai_con)) "0, 0,15.000000") 1.5e+03 (Variables|Default|GetDesiredObjectTypes) false (Utilities|Array|MakeArray (Pawn|GetControlledPawn (Variables|Default|GetAI_CON_Ref))) "None"))
  (bind _array_element (Utilities|Array|ForEachLoopwithBreak _outhits)
    (:LoopBody
      (bind _outhit (Collision|LineTraceByChannel 0 (Variables|Default|GetMy%20Location) (Transformation|GetActorLocation (.HitActor (Collision|BreakHitResult _array_element))) "TraceTypeQuery2" false (Utilities|Array|MakeArray (Pawn|GetControlledPawn (Variables|Default|GetAI_CON_Ref))) "None"))
      (if (== (.HitActor (Collision|BreakHitResult _outhit)) (.HitActor (Collision|BreakHitResult _array_element)))
        (Class|BTFunctionLibrary|SetBlackboardValueasObject (Variables|Default|GetTargetToFollow) (.HitActor (Collision|BreakHitResult _outhit)))
        (AI|BehaviorTree|SetBlackboardValueasVector (Variables|Default|GetTargetLocation) (Transformation|GetActorLocation (.HitActor (Collision|BreakHitResult _outhit))))
        (else
          (Class|BTFunctionLibrary|SetBlackboardValueasObject (Variables|Default|GetTargetToFollow)))))))