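; Player character Blueprint with control-relative movement, "piece"-tagged lantern pickups and a pause menu.
; Pickup input stores the last overlapped actor's owner in Pieces, then destroys that actor.
; Holding CollectClus runs a Delay loop up to a three-second, never-reset HoldTime, then destroys tagged AI_Character actors without any proximity check.
; Construction creates a dynamic energy material and records initial EnergyLevel, but the energy drain logic is disconnected.
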(event EventTick
  (params (DeltaSeconds :type Float%20%28single-precision%29)))

(event EventActorBeginOverlap
  (params (OtherActor :type Actor%20Object%20Reference))
  ;[1 1 1] Lantern Piece Pickup
)

(event Input|ActionEvents|InputActionCollectClus
  ;[1 1 1] Clu Pickup
  (:Pressed
    (Variables|Default|SetisCollectingClus true)
    (bind _outactors (Actor|GetAllActorsOfClass 0 "/Game/Blueprints/AI_Character.AI_Character_C"))
    (for _array_element _outactors
      (bind _asai_character (Utilities|Casting|CastToAI_Character _array_element))
      (if (Variables|Default|GetisCollectingClus)
        (if (>= (Variables|Default|GetholdTime) 3.0) :!label _label
          (Development|PrintString 0 "Finished Delaying")
          (if (Actor|ActorHasTag _asai_character (Utilities|Array|Get(acopy) (Variables|/Script/Engine.Actor|GetTags _asai_character)))
            (Actor|DestroyActor _asai_character))
          (else
            (Variables|Default|SetholdTime (+ (Variables|Default|GetholdTime) 1.0))
            (Utilities|FlowControl|Delay 0 1.0)
            (Development|PrintString 0 "still delaying")
            (if (Variables|Default|GetisCollectingClus)
              (goto _label)))))))
  (:Released
    (Variables|Default|SetisCollectingClus false)))

(event Input|ActionEvents|InputActionCollectPickup
  ;[1 1 1] Lantern Piece Pickup
  (:Pressed
    (if (Utilities|Name|Equal(Name) (Utilities|Array|Get(acopy) (Variables|/Script/Engine.Actor|GetTags (stale EventActorBeginOverlap OtherActor))) "piece")
      (bind _returnvalue (Utilities|Array|Add (Variables|Default|Getpieces) (Components|GetOwner (stale EventActorBeginOverlap OtherActor))))
      (Development|PrintString (Utilities|String|ToString(Integer) _returnvalue))
      (Actor|DestroyActor (stale EventActorBeginOverlap OtherActor))
      (else
        (Development|PrintString 0 "Nah")))))

(event Input|ActionEvents|InputActionMenu
  ;[1 1 1] Pause Menu
  (:Pressed
    (Game|SetGamePaused 0 true)
    (bind _returnvalue (UserInterface|CreateWidget "/Game/Pause.Pause_C"))
    (UserInterface|Viewport|AddtoViewport _returnvalue)
    (Variables|/Script/Engine.PlayerController|SetbShowMouseCursor (Game|GetPlayerController 0) true)))

(event Input|AxisEvents|InputAxisMoveRight
  (params (AxisValue :type Float%20%28single-precision%29))
  ;[1 1 1] Movement (With WASD)
  (Pawn|Input|AddMovementInput (Math|Vector|GetRightVector (Pawn|GetControlRotation :!class /Script/Engine.Pawn)) AxisValue false))

(event Input|AxisEvents|InputAxisMoveForward
  (params (AxisValue :type Float%20%28single-precision%29))
  ;[1 1 1] Movement (With WASD)
  (Pawn|Input|AddMovementInput (Math|Vector|GetForwardVector (Pawn|GetControlRotation :!class /Script/Engine.Pawn)) AxisValue false))

(fn ConstructionScript
  (bind _returnvalue (Rendering|Material|CreateDynamicMaterialInstance (Variables|Character|GetMesh) 0 "/Game/Materials/CharacterMaterial_Inst.CharacterMaterial_Inst" :!class /Script/Engine.PrimitiveComponent))
  (Variables|Default|SetDynamic%20Energy%20Mat _returnvalue)
  (Variables|Default|SetIntial%20Energy%20Level (Math|Conversions|ToFloat(Integer) (Variables|Default|GetenergyLevel))))