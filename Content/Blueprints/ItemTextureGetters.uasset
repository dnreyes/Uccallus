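; ItemTextureGetters provides lookup functions that return icon textures for piece and gem types.
; GetPieceIconByType switches on math-themed piece types; only Add and Constant have their own textures, while every other type returns the minus icon.
; GetGemIconByType maps each gem type to its own UI crystal texture.
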(fn GetPieceIconbyType
  (params (PieceType :type EPieceType%20Enum :default "P_Add"))
  (switch Utilities|FlowControl|Switch|SwitchonEPieceType PieceType
    (:P_Add
      (LocalVariables|SetResult "/Game/Textures/piece_plus.piece_plus"))
    (:P_Subtract
      (LocalVariables|SetResult "/Game/Textures/piece_minus.piece_minus"))
    (:P_Multiply
      (LocalVariables|SetResult "/Game/Textures/piece_minus.piece_minus"))
    (:P_Exponent
      (LocalVariables|SetResult "/Game/Textures/piece_minus.piece_minus"))
    (:P_Var
      (LocalVariables|SetResult "/Game/Textures/piece_minus.piece_minus"))
    (:P_Const
      (LocalVariables|SetResult "/Game/Textures/T_LampPiece.T_LampPiece"))
    (:P_Log
      (LocalVariables|SetResult "/Game/Textures/piece_minus.piece_minus"))
    (:P_Sqrt
      (LocalVariables|SetResult "/Game/Textures/piece_minus.piece_minus"))
    (:P_Half
      (LocalVariables|SetResult "/Game/Textures/piece_minus.piece_minus")))
  (return (LocalVariables|GetResult)))

(fn GetGemIconbyType
  (params (GemType :type EGemType%20Enum :default "G_Yellow"))
  (switch Utilities|FlowControl|Switch|SwitchonEGemType GemType
    (:G_Clear
      (LocalVariables|SetResult "/Game/Textures/UI-glass-crystal.UI-glass-crystal"))
    (:G_Yellow
      (LocalVariables|SetResult "/Game/Textures/UI-yellow-crystal.UI-yellow-crystal"))
    (:G_Blue
      (LocalVariables|SetResult "/Game/Textures/UI-blue-crystal.UI-blue-crystal"))
    (:G_Red
      (LocalVariables|SetResult "/Game/Textures/UI-red-crystal.UI-red-crystal"))
    (:G_Diamond
      (LocalVariables|SetResult "/Game/Textures/UI-diamond-crystal.UI-diamond-crystal")))
  (return (LocalVariables|GetResult)))