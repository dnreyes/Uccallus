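; Lantern Blueprint holding an unfinished mechanic for crystallizing Clus, with none of its logic connected to a running event.
; The disconnected graph checks for at least one Clu, then prints and stores the decremented count, or prints a shortage warning.
; CrystallizeClu returns the decremented count as a string, which the graph converts back to an integer.
; CheckCluCount, Tick and the construction script are empty, and a gem value read is unused.
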(event EventTick
  (params (DeltaSeconds :type Float%20%28single-precision%29)))

(event Input|ActionEvents|InputActionCreateCluGem)

(fn ConstructionScript)

(fn CrystallizeClu
  (return (Utilities|String|ToString(Integer) (- (Variables|Default|GetcluCount) 1))))

(fn CheckCluCount)