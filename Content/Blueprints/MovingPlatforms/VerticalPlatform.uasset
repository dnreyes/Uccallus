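; VerticalPlatform is a touch-activated moving platform that, despite its name, shifts along world X.
; Touching it runs IsEquationValid, which prints whether the hero's PieceCollection holds exactly one piece, but Activate runs regardless of the result.
; Activate uses a Delay and Gate loop to step the actor with VInterpTo toward a point recomputed just ahead of its current location, which also feeds the gate's stop check.
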(event EventActivate
  (bind _returnvalue (Transformation|GetActorLocation))
  (bind (_x _y _z) (Math|Vector|BreakVector _returnvalue))
  (bind _returnvalue_2 (+ _x 1e+01))
  (bind _returnvalue_3 (Math|Vector|MakeVector _returnvalue_2 _y _z))
  (Utilities|FlowControl|Sequence
    (:then_0
      (Transformation|SetActorLocation (Math|Interpolation|VInterpTo _returnvalue _returnvalue_3 (Utilities|Time|GetWorldDeltaSeconds) 0.0) false :!label _label)
      (Utilities|FlowControl|Delay 0.1)
      (Utilities|FlowControl|Sequence
        (:then_0
          (Utilities|FlowControl|Gate true :!label _label_2
            (:Exit
              (goto _label))))
        (:then_1
          (if (Math|Vector|Equal(Vector) _returnvalue _returnvalue_3 1e+01)
            (goto _label_2 Close)
            (else
              (goto _label_2 Open))))))
    (:then_1
      (goto _label_2 Open))))

(event EventBeginPlay
  (Input|EnableInput (Game|GetPlayerController 0)))

(event EventActorOnInputTouchBegin
  (params (FingerIndex :type ETouchIndex%20Enum :default "Touch1"))
  (bind _returnvalue (CallFunction|IsEquationValid))
  (if _returnvalue
    _
    (else
      _))
  (Class|Pedestal|Activate))

(fn ConstructionScript)

(fn IsEquationValid
  (bind _herocharacter (Variables|Default|GetHeroCharacter))
  (bind _piececollection (Variables|/Script/Uccallus.UccallusCharacter|GetPieceCollection _herocharacter))
  (bind _returnvalue (Utilities|Array|Length _piececollection))
  (Development|PrintString (Utilities|String|ToString(Integer) _returnvalue))
  (if (== _returnvalue 1)
    (bind _output_get (LocalVariables|SetbIsValid true))
    (Development|PrintString (Utilities|String|ToString(Boolean) _output_get))
    (else
      (bind _output_get_2 (LocalVariables|SetbIsValid false))
      (Development|PrintString (Utilities|String|ToString(Boolean) _output_get_2))))
  (return (LocalVariables|GetbIsValid)))