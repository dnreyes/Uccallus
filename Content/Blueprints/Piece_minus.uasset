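; Collectible minus-sign piece that the player picks up into the HUD's pieces inventory, with its ID, mesh and inventory struct set at construction.
; Trigger overlap registers it with MyCharacter, toggles a pickup prompt widget and tracks range.
; The character's OnPickupItem dispatcher runs PiecePickup when in range, which adds the piece or bumps its count, hides it, disables collision and refreshes the inventory.
; CheckLantern always returns false.
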(event OnComponentBeginOverlap(Trigger)
  (params (OtherActor :type Actor%20Object%20Reference) (OtherComp :type Primitive%20Component%20Object%20Reference) (OtherBodyIndex :type Integer) (bFromSweep :type Boolean) (SweepResult :type Hit%20Result%20Structure%20%28by%20ref%29))
  ;[1 1 1] Is In Range Trigger
  (bind _asmy_character (Utilities|Casting|CastToMyCharacter OtherActor))
  (Default|AddtoInventory _asmy_character self)
  (UserInterface|Viewport|AddtoViewport (Variables|Default|GetPickupTextWidget) 0)
  (Variables|Default|SetIsInRange true))

(event OnComponentEndOverlap(Trigger)
  (params (OtherActor :type Actor%20Object%20Reference) (OtherComp :type Primitive%20Component%20Object%20Reference) (OtherBodyIndex :type Integer))
  ;[1 1 1] Is In Range Trigger
  (Utilities|Casting|CastToMyCharacter OtherActor)
  (Widget|RemovefromParent (Variables|Default|GetPickupTextWidget))
  (Variables|Default|SetIsInRange false))

(event Custom|OnPickupItem_Event_1
  ;[1 1 1] Item Pickup
  (if (and (Collision|GetActorEnableCollision) (Variables|Default|GetIsInRange))
    (CallFunction|PiecePickup)))

(event EventBeginPlay
  (bind _iteminfo (Variables|Default|GetItemInfo))
  (bind (_item _icon _count _pickuptext) (Utilities|Struct|BreakInventoryStruct _iteminfo))
  ;[1 1 1] Initialize Pickup
  (bind _returnvalue (UserInterface|CreateWidget "/Game/UMG/PickupText.PickupText_C"))
  (bind _output_get (Variables|Default|SetPickupTextWidget _returnvalue))
  (Variables|/Game/UMG/PickupText.PickupText_C|SetPickupActor _output_get _item)
  (Variables|/Game/UMG/PickupText.PickupText_C|SetPickupText _output_get _pickuptext)
  (Utilities|Struct|SetmembersinInventoryStruct _iteminfo self)
  (bind _asmy_character (Utilities|Casting|CastToMyCharacter (Game|GetPlayerCharacter 0)))
  (bind _output_get_2 (Variables|Default|SetHeroCharacter _asmy_character))
  (EventDispatchers|AssignOnPickupItem _output_get_2 (delegate Custom|OnPickupItem_Event_1)))

(fn ConstructionScript
  ;[1 1 1] Inital Piece Set UP
  (Variables|Default|Setid "-")
  (Variables|Default|SetcheckInput false)
  ;[1 1 1] Set Up for Inventory
  (Utilities|Struct|SetmembersinInventoryStruct (Variables|Default|GetItemInfo) self (Variables|Default|GetIcon) 0 (Variables|Default|GetPickupText))
  (Components|StaticMesh|SetStaticMesh (Variables|Default|GetCustomMesh)))

(fn PiecePickup
  (bind _herocharacter (Variables|Default|GetHeroCharacter))
  (bind _iteminfo (Variables|Default|GetItemInfo))
  (bind _gamehudwidget (Variables|/Game/Blueprints/MyCharacter.MyCharacter_C|GetGameHUDWidget _herocharacter))
  (bind _piecesinventory (Variables|/Game/UMG/GameHUD.GameHUD_C|GetPiecesInventory _gamehudwidget))
  (if (Math|Boolean|NotEqual(Boolean) (Utilities|Array|ContainsItem _piecesinventory _iteminfo) true)
    (Utilities|Array|Add _piecesinventory _iteminfo)
    (else
      (Utilities|Struct|SetmembersinInventoryStruct _iteminfo 0 0 (+ (.Count (Utilities|Struct|BreakInventoryStruct _iteminfo)) 1))))
  (Widget|RemovefromParent (Variables|Default|GetPickupTextWidget))
  (Rendering|SetActorHiddenInGame true)
  (Collision|SetActorEnableCollision false)
  (Default|RefreshInventory _gamehudwidget))

(fn CheckLantern
  (params (id :type String))
  (return false))